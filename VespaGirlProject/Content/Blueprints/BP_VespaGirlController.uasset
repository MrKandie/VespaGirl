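; BP_VespaGirlController handles steering and acceleration input for what its name indicates is a Vespa-riding girl character.
; The Turn axis adds controller yaw scaled by TurnScale.
; The Accelerate axis adds forced movement input along the forward vector of the full control rotation, scaled by AccelerateScale, so steering sets the travel direction.
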(event `InputAxis|Turn`
  (params (AxisValue :type "Float (single-precision)"))
  ;[1 1 1] Turn
  (`self.AddControllerYawInput` (* AxisValue (`self.TurnScale`))))

(event `InputAxis|Accelerate`
  (params (AxisValue :type "Float (single-precision)"))
  ;[1 1 1] Acceleration
  (`self.AddMovementInput` (`KismetMathLibrary.GetForwardVector` (`self.GetControlRotation`)) (* AxisValue (`self.AccelerateScale`)) true))

(fn `UserConstructionScript`)